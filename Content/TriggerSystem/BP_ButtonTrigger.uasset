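; Pressure button trigger that activates when something overlaps its sphere and lowers its mesh with a timeline, reversing it on release.
; Unless persistent, it releases after a timer if a deactivation time is set, otherwise after a delay when the overlap ends.
; Each state change either calls Activate on its triggerable actors when flagged as last, or fires a state-changed dispatcher.
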(event `self.SphereTrigger.OnComponentBeginOverlap`
  (params (OverlappedComponent :type "PrimitiveComponent Object Reference") (OtherActor :type "Actor Object Reference") (OtherComp :type "PrimitiveComponent Object Reference") (OtherBodyIndex :type Integer) (bFromSweep :type Boolean) (SweepResult :type "HitResult Structure (by ref)"))
  ;[0.6094 0.6094 0.6094] Player Interaction with Trigger
  (if (not (`self.IsActive`))
    (if (> (`self.DeactivationTime`) 0.0)
      (bind _returnvalue (`KismetSystemLibrary.K2_SetTimerDelegate` (`|CreateDelegate` :!event `StartDeactivateWithTimer`) (`self.DeactivationTime`)))
      (set `self.Timer` _returnvalue))
    (set `self.IsActive` true)
    (`|ExecutionSequence` :!label _label
      (:`then_0`
        (switch `int` (`KismetMathLibrary.Conv_BoolToInt` (`self.IsActive`))
          (:`0`
            (bind (_direction _movepercent) (`Timeline|ChangeMeshHeightTimeline` :`NewTime` 1.0 :!via `ReverseFromEnd` :!label _label_2)
              (:`Update`
                (`SceneComponent.K2_SetRelativeLocation` (`self.StaticMesh`) (`KismetMathLibrary.MakeVector` 0.0 0.0 (`KismetMathLibrary.Lerp` 0.0 -7.0 _movepercent)) false false))))
          (:`1`
            (goto _label_2 :!via `PlayFromStart`))))
      (:`then_1`
        (if (`self.IsLast`)
          (for _array_element (`self.TrigerableActors`)
            (`/Game/TriggerSystem/BP_BaseTriggerableActor.Activate` _array_element (`self.IsActive`)))
          (else
            (`self.StateChangedDispatcher`)))))))

(event `StartDeactivateWithTimer`
  ;[0.6094 0.6094 0.6094] Player Interaction with Trigger
  (`KismetSystemLibrary.K2_ClearAndInvalidateTimerHandle` (`self.Timer`))
  (if (not (`self.isPersistent`)) :!label _label_3
    (set `self.IsActive` false)
    (goto _label)))

(event `self.SphereTrigger.OnComponentEndOverlap`
  (params (OverlappedComponent :type "PrimitiveComponent Object Reference") (OtherActor :type "Actor Object Reference") (OtherComp :type "PrimitiveComponent Object Reference") (OtherBodyIndex :type Integer))
  ;[0.6094 0.6094 0.6094] Player Interaction with Trigger
  (if (<= (`self.DeactivationTime`) 0.0)
    (`KismetSystemLibrary.Delay` (`self.DeactivateDelay`))
    (goto _label_3)))

(fn `UserConstructionScript`
  (`parent.UserConstructionScript`))