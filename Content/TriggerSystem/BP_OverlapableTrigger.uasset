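; BP_OverlapableTrigger is a trigger actor that becomes active when its Box component is overlapped.
; When IsLast is set it passes state changes to TrigerableActors through Activate, otherwise it calls the state-changed dispatcher.
; A positive DeactivationTime starts a one-shot timer on activation, apparently for deactivation; otherwise ending the overlap deactivates it.
; IsPersistent blocks deactivation, keeping the trigger active.
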(event `self.Box.OnComponentBeginOverlap`
  (params (OverlappedComponent :type "PrimitiveComponent Object Reference") (OtherActor :type "Actor Object Reference") (OtherComp :type "PrimitiveComponent Object Reference") (OtherBodyIndex :type Integer) (bFromSweep :type Boolean) (SweepResult :type "HitResult Structure (by ref)"))
  (if (not (`self.IsActive`))
    (if (> (`self.DeactivationTime`) 0.0)
      (bind _returnvalue (`KismetSystemLibrary.K2_SetTimerDelegate` (`|CreateDelegate` :!event `StartDeactivateWithTimer`) (`self.DeactivationTime`)))
      (set `self.Timer` _returnvalue))
    (set `self.IsActive` true)
    (if (`self.IsLast`) :!label _label
      (for _array_element (`self.TrigerableActors`)
        (`/Game/TriggerSystem/BP_BaseTriggerableActor.Activate` _array_element (`self.IsActive`)))
      (else
        (`self.StateChangedDispatcher`)))))

(event `StartDeactivateWithTimer`
  (`KismetSystemLibrary.K2_ClearAndInvalidateTimerHandle` (`self.Timer`))
  (if (not (`self.isPersistent`)) :!label _label_2
    (set `self.IsActive` false)
    (goto _label)))

(event `self.Box.OnComponentEndOverlap`
  (params (OverlappedComponent :type "PrimitiveComponent Object Reference") (OtherActor :type "Actor Object Reference") (OtherComp :type "PrimitiveComponent Object Reference") (OtherBodyIndex :type Integer))
  (if (<= (`self.DeactivationTime`) 0.0)
    (goto _label_2)))

(fn `UserConstructionScript`
  (`parent.UserConstructionScript`))