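; BP_TriggerableDoor is a triggerable door that opens or closes in response to its inherited Activate event.
; Activate calls the parent, then plays the OpenAndCloseDoor timeline to open or reverses it to close.
; The timeline's RotationAmount track drives both location and rotation lerps on the StaticMesh, from zero relative transform toward OpenLocation and OpenRotation, so the door can slide, swing or both.
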(event `self.Activate`
  (params (ShouldActivate :type Boolean))
  (`parent.Activate` ShouldActivate)
  (if ShouldActivate
    (bind (_direction _rotationamount) (`Timeline|OpenAndCloseDoor` :!label _label)
      (:`Update`
        (`SceneComponent.K2_SetRelativeLocationAndRotation` (`self.StaticMesh`) (`KismetMathLibrary.VLerp` (0.0 0.0 0.0) (`self.OpenLocation`) _rotationamount) (`KismetMathLibrary.RLerp` (struct) (`self.OpenRotation`) _rotationamount) false false)))
    (else
      (goto _label :!via `Reverse`))))

(fn `UserConstructionScript`
  (`parent.UserConstructionScript`))