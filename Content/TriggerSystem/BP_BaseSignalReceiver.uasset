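; Base signal receiver for the trigger system, acting as a logic gate that combines the states of several signal generators.
; On BeginPlay it binds to each generator's state-changed dispatcher and re-evaluates on every signal, handling only the AND type, which requires all generators active.
; The last receiver passes the result to its triggerable actors' Activate, while others fire their own state-changed dispatcher, allowing chained gates.
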(event `self.ReceiveBeginPlay`
  (for _array_element (`self.SignalGenerators`)
    (add `self.StateChangedDispatcher` _array_element (delegate `OnStateChangedSignalReceived`))))

(event `OnStateChangedSignalReceived`
  (switch `/Game/TriggerSystem/E_RecieverType` (`self.RecieverType`)
    (:`NewEnumerator0`
      (`self.HandleAndSignal`))))

(fn `HandleAndSignal`
  (locals (AllGeneratorsAreActive :type Boolean))
  ;[1 1 1] Check AND Gate State - Complete if the AND Gate is true and break if the AND condition is false.
  (set `local.AllGeneratorsAreActive` true)
  (for _array_element (`self.SignalGenerators`)
    (if (not (`/Game/TriggerSystem/BP_BaseSignalGenerator.IsActive` _array_element))
      (set `local.AllGeneratorsAreActive` false)
      (break)))
  ;[1 1 1] Handle the AND Gate States
  (set `self.IsActive` (`local.AllGeneratorsAreActive`))
  (if (`self.IsLast`)
    (for _array_element_2 (`self.TrigerableActors`)
      (`/Game/TriggerSystem/BP_BaseTriggerableActor.Activate` _array_element_2 (`self.IsActive`)))
    (else
      (`self.StateChangedDispatcher`))))

(fn `UserConstructionScript`
  (`parent.UserConstructionScript`))